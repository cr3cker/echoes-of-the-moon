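; Interaction component that lets its owning actor detect nearby interactable actors, show their look-at message and interact with them on input.
; On BeginPlay it creates a WB_Interact widget, then every Tick runs a sphere trace at the owner's location.
; A hit actor implementing BPI_Interact becomes the current target and supplies the widget text; otherwise both are cleared.
; The IA_Interaction input calls InteractWithMessage on that target, passing the owner.
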(event `self.ReceiveBeginPlay`
  (`self.CreateInteractDisplay`))

(event `self.ReceiveTick`
  (params (DeltaSeconds :type "Float (single-precision)"))
  (`self.InteractionTrace`))

(event `CreateInteractDisplay`
  ;[1 1 1] Create interaction display
  (bind _returnvalue (`|CreateWidget` "/Game/UI/InteractUI/WB_Interact.WB_Interact_C"))
  (bind _output_get (set `self.InteractDisplay` _returnvalue))
  (`UserWidget.AddToViewport` _output_get 0))

(event `EnhancedInput|/Game/ThirdPerson/Input/Actions/IA_Interaction`
  (params (ActionValue :type Boolean) (ElapsedSeconds :type "Float (double-precision)") (TriggeredSeconds :type "Float (double-precision)") (InputAction :type "InputAction Object Reference" :default "/Game/ThirdPerson/Input/Actions/IA_Interaction.IA_Interaction"))
  ;[1 1 1] Interaction Input
  (:`Started`
    (bind _hittarget (`self.HitTarget`)
      (:`then`
        (message `/Game/InteractionSystem/BPI_Interact.InteractWith` _hittarget (`self.GetOwner`)))
      (:`else`))))

(fn `InteractionTrace`
  (bind _returnvalue (`Actor.K2_GetActorLocation` (`self.GetOwner`)))
  (bind (_outhit _returnvalue_2) (`KismetSystemLibrary.SphereTraceSingle` _returnvalue _returnvalue (`self.Radius`) "TraceTypeQuery3"))
  (if _returnvalue_2
    (bind (_bblockinghit _binitialoverlap _time _distance _location _impactpoint _normal _impactnormal _physmat _hitactor) (`GameplayStatics.BreakHitResult` _outhit))
    (if (`KismetSystemLibrary.DoesImplementInterface` _hitactor "/Game/InteractionSystem/BPI_Interact.BPI_Interact_C")
      (bind _output_get (set `self.HitTarget` _hitactor))
      (bind _interacttext (message `/Game/InteractionSystem/BPI_Interact.LookAt` _output_get))
      (`/Game/UI/InteractUI/WB_Interact.UpdateInteractText` (`self.InteractDisplay`) _interacttext)
      (else
        (set `self.HitTarget` null)
        (`/Game/UI/InteractUI/WB_Interact.UpdateInteractText` (`self.InteractDisplay`) "")))
    (else
      (set `self.HitTarget` null)
      (`/Game/UI/InteractUI/WB_Interact.UpdateInteractText` (`self.InteractDisplay`) ""))))