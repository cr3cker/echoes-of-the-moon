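; BP_CutScene_ALtar is a trigger actor that plays the altar cutscene and ends the game.
; When BP_ThirdPersonCharacter_forest overlaps its Box, it creates a Level Sequence player, puts BP_PlayerController into cutscene mode and starts playback.
; It calls EndOfTheGame on the controller right after Play, without waiting for the sequence to finish.
; CutScenePlayed is only ever set to false, so it never records that the scene played.
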(event `self.Box.OnComponentBeginOverlap`
  (params (OverlappedComponent :type "PrimitiveComponent Object Reference") (OtherActor :type "Actor Object Reference") (OtherComp :type "PrimitiveComponent Object Reference") (OtherBodyIndex :type Integer) (bFromSweep :type Boolean) (SweepResult :type "HitResult Structure (by ref)"))
  (cast `/Game/ThirdPerson/Blueprints/BP_ThirdPersonCharacter_forest` OtherActor)
  (bind (_outactor _returnvalue) (`LevelSequencePlayer.CreateLevelSequencePlayer` (`self.CutScene`)))
  (if (`self.CutScenePlayed?`)
    _
    (else
      _))
  (bind _asbp_player_controller (cast `/Game/ThirdPerson/Blueprints/BP_PlayerController` (`GameplayStatics.GetPlayerController` 0)))
  (`/Game/ThirdPerson/Blueprints/BP_PlayerController.StartCutSceneMode` _asbp_player_controller)
  (`MovieSceneSequencePlayer.Play` _returnvalue)
  (set `self.CutScenePlayed?` false)
  (bind _asbp_player_controller_2 (cast `/Game/ThirdPerson/Blueprints/BP_PlayerController` (`GameplayStatics.GetPlayerController` 0)))
  (`/Game/ThirdPerson/Blueprints/BP_PlayerController.EndOfTheGame` _asbp_player_controller_2))

(fn `UserConstructionScript`)