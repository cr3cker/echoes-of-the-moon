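; Altar cutscene trigger that rewards collecting three ducks, read from the game instance when something overlaps its box.
; It starts the target gate's event, then for the player character plays a level sequence and completes the side quest.
; A played flag, set with the cutscene, blocks repeats.
; The controller's cutscene mode ends right after playback starts, without waiting for the sequence to finish.
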(event `self.Box.OnComponentBeginOverlap`
  (params (OverlappedComponent :type "PrimitiveComponent Object Reference") (OtherActor :type "Actor Object Reference") (OtherComp :type "PrimitiveComponent Object Reference") (OtherBodyIndex :type Integer) (bFromSweep :type Boolean) (SweepResult :type "HitResult Structure (by ref)"))
  (if (not (`self.CutScenePlayed?`))
    (bind _asbp_my_game_instance (cast `/Game/ThirdPerson/Blueprints/BP_MyGameInstance` (`GameplayStatics.GetGameInstance`)))
    (if (== (`/Game/ThirdPerson/Blueprints/BP_MyGameInstance.DucksCollected` _asbp_my_game_instance) 3)
      (`|ExecutionSequence`
        (:`then_0`
          (`/Game/Blueprints/BP_LevelAcess.StartGateEvent` (`self.TargetGate`)))
        (:`then_1`
          (cast `/Game/ThirdPerson/Blueprints/BP_ThirdPersonCharacter` OtherActor)
          (bind (_outactor _returnvalue) (`LevelSequencePlayer.CreateLevelSequencePlayer` (`self.CutScene`)))
          (if (`self.CutScenePlayed?`)
            _
            (else
              _))
          (bind _asbp_player_controller (cast `/Game/ThirdPerson/Blueprints/BP_PlayerController` (`GameplayStatics.GetPlayerController` 0)))
          (`/Game/ThirdPerson/Blueprints/BP_PlayerController.StartCutSceneMode` _asbp_player_controller)
          (`MovieSceneSequencePlayer.Play` _returnvalue)
          (set `self.CutScenePlayed?` true)
          (cast `/Game/ThirdPerson/Blueprints/BP_PlayerController` (`GameplayStatics.GetPlayerController` 0))
          (`/Game/ThirdPerson/Blueprints/BP_PlayerController.EndCutSceneMode` _asbp_player_controller))
        (:`then_2`
          (bind _asbp_third_person_character (cast `/Game/ThirdPerson/Blueprints/BP_ThirdPersonCharacter` OtherActor))
          (`/Game/ThirdPerson/Blueprints/BP_ThirdPersonCharacter.SideQuestComplete` _asbp_third_person_character))))))

(fn `UserConstructionScript`)