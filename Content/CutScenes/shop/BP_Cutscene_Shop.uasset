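; BP_Cutscene_Shop is a trigger actor that plays a shop cutscene when the third-person character overlaps its box.
; If CutScenePlayed is true, it creates a Level Sequence player, has the player controller hide the UI and enter cutscene mode, then plays.
; The sequence's finish event ends cutscene mode.
; The node clearing CutScenePlayed is disconnected, so nothing here prevents replays on later overlaps.
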(event `self.Box.OnComponentBeginOverlap`
  (params (OverlappedComponent :type "PrimitiveComponent Object Reference") (OtherActor :type "Actor Object Reference") (OtherComp :type "PrimitiveComponent Object Reference") (OtherBodyIndex :type Integer) (bFromSweep :type Boolean) (SweepResult :type "HitResult Structure (by ref)"))
  (cast `/Game/ThirdPerson/Blueprints/BP_ThirdPersonCharacter` OtherActor)
  (if (`self.CutScenePlayed?`)
    (bind (_outactor _returnvalue) (`LevelSequencePlayer.CreateLevelSequencePlayer` (`self.Cutscene`)))
    (add `MovieSceneSequencePlayer.OnFinished` _returnvalue (delegate `OnFinished_Event`))
    (bind _asbp_player_controller (cast `/Game/ThirdPerson/Blueprints/BP_PlayerController` (`GameplayStatics.GetPlayerController` 0)))
    (`/Game/ThirdPerson/Blueprints/BP_PlayerController.HideUI` _asbp_player_controller)
    (`/Game/ThirdPerson/Blueprints/BP_PlayerController.StartCutSceneMode` _asbp_player_controller)
    (`MovieSceneSequencePlayer.Play` _returnvalue)))

(event `OnFinished_Event`
  (bind _asbp_player_controller (cast `/Game/ThirdPerson/Blueprints/BP_PlayerController` (`GameplayStatics.GetPlayerController` 0)))
  (`/Game/ThirdPerson/Blueprints/BP_PlayerController.EndCutSceneMode` _asbp_player_controller))

(fn `UserConstructionScript`)