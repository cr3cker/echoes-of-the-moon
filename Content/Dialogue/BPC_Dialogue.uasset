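; Dialogue component that lets its owning actor hold a conversation when interacted with, using an on-screen dialogue widget.
; The first interaction creates the display with a name and portrait and sets the owner's BP_AIController to conversing with the interactor.
; Further interactions signal the dialogue box that the speaker finished.
; EndDialogue removes the widget and returns the AI to idle, while LookAt returns empty text.
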(event `self.ReceiveBeginPlay`
  (bind _asbp_aicontroller (cast `/Game/Dialogue/AI/BP_AIController` (`AIBlueprintHelperLibrary.GetAIController` (`self.GetOwner`))))
  (set `self.AIController` _asbp_aicontroller))

(event `CreateDialogueDisplay`
  (`self.DialogueDisplay`
    (:`then`
      (`/Game/UI/DialogueUI/WB_DIalogueBox.OnSpeakerFinished` (`/Game/UI/DialogueUI/WB_DialogueDisplay.DIalogueBox` (`self.DialogueDisplay`))))
    (:`else`
      (bind _returnvalue (`|CreateWidget` "/Game/UI/DialogueUI/WB_DialogueDisplay.WB_DialogueDisplay_C" null (`self.Name`) (`self.Portrait`)))
      (bind _output_get (set `self.DialogueDisplay` _returnvalue))
      (`UserWidget.AddToViewport` _output_get 0)
      (bind _aicontroller (`self.AIController`)
        (:`then`
          (`/Game/Dialogue/AI/BP_AIController.SetStateAsConversating` _aicontroller (`self.Interactor`)))
        (:`else`)))))

(event `/Game/InteractionSystem/BPI_Interact.InteractWith`
  (params (Interactor :type "Actor Object Reference"))
  (set `self.Interactor` Interactor)
  (`self.CreateDialogueDisplay`))

(event `EndDialogue`
  ;[1 1 1] End dialogue logic
  (bind _dialoguedisplay (`self.DialogueDisplay`)
    (:`then`
      (`Widget.RemoveFromParent` _dialoguedisplay)
      (set `self.DialogueDisplay` null)
      (bind _aicontroller (`self.AIController`)
        (:`then`
          (`/Game/Dialogue/AI/BP_AIController.SetStateAsIdle` _aicontroller))
        (:`else`)))
    (:`else`)))

(fn `LookAt`
  (returns (InteractText :type Text))
  (return ""))