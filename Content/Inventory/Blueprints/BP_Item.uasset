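; BP_Item is an inventory item actor placed in the world, displayed with the mesh from its Item data.
; The construction script applies that mesh to the StaticMesh component and disables physics simulation.
; On BeginPlay it destroys itself if BP_MyGameInstance lists its ActorID in DestroyedActorIDs, so items recorded as destroyed do not reappear.
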(event `self.ReceiveBeginPlay`
  (bind _asbp_my_game_instance (cast `/Game/ThirdPerson/Blueprints/BP_MyGameInstance` (`GameplayStatics.GetGameInstance`)))
  (if (`KismetArrayLibrary.Array_Contains` (`/Game/ThirdPerson/Blueprints/BP_MyGameInstance.DestroyedActorIDs` _asbp_my_game_instance) (`self.ActorID`))
    (`self.K2_DestroyActor`)))

(fn `UserConstructionScript`
  (bind _staticmesh (`self.StaticMesh`))
  (`StaticMeshComponent.SetStaticMesh` _staticmesh (`.Mesh_16_6D9F3521CAAD4133BEF3723DB38B9297` (break `/Game/Inventory/Blueprints/S_Itemstructure` (`self.Item`))))
  (`PrimitiveComponent.SetSimulatePhysics` _staticmesh false))