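; Moon Beetle enemy AI that chases pawns seen through PawnSensing and plays an attack montage on reaching them.
; A retriggerable delay acts as lost-sight timeout, fading chase music that a GameMode flag keeps from overlapping.
; BPCDamageSystem handles health and triggers Death, which, only if chase music is valid, destroys the beetle and counts kills, completing a quest at three.
; A left-click slash with debug sphere trace is also present.
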(event `self.ReceiveBeginPlay`
  (bind _asbp_third_person_game_mode_2 (cast `/Game/ThirdPerson/Blueprints/BP_ThirdPersonGameMode2` (`GameplayStatics.GetGameMode`)))
  (set `self.As BP Third Person Game Mode 2` _asbp_third_person_game_mode_2))

(event `ChasePlayer`
  (params (TargetPawn :type "Pawn Object Reference"))
  (`|AIMoveTo` self (0.0 0.0 0.0) TargetPawn 260.0
    (:`OnSuccess`
      (if (`self.canAttack?`)
        (`|PlayMontage` (`self.Mesh`) "/Game/assets/characters/lienka/animations/A_Attack_Montage.A_Attack_Montage" 1.5
          (:`then`
            (set `self.canAttack?` false))
          (:`OnCompleted`
            (set `self.canAttack?` true :!label _label))
          (:`OnInterrupted`
            (goto _label)))))))

(event `self.PawnSensing.OnSeePawn`
  (params (Pawn :type "Pawn Object Reference"))
  (bind _as_bp_third_person_game_mode_2 (`self.As BP Third Person Game Mode 2`))
  (`|ExecutionSequence`
    (:`then_0`
      (`self.ChasePlayer` Pawn)
      (`|ExecutionSequence`
        (:`then_0`
          (`/Engine/EditorBlueprintResources/StandardMacros.DoOnce` false :!label _label_2
            (:`Completed`
              (if (not (`/Game/ThirdPerson/Blueprints/BP_ThirdPersonGameMode2.MusicPlaying?` _as_bp_third_person_game_mode_2))
                (set `/Game/ThirdPerson/Blueprints/BP_ThirdPersonGameMode2.MusicPlaying?` true _as_bp_third_person_game_mode_2)
                (bind _returnvalue (`GameplayStatics.SpawnSound2D` "/Game/Sounds/SoundSystem/AIChase.AIChase" 1.0 1.0 0.0 null))
                (set `self.AIChaseMusic` _returnvalue)))))
        (:`then_1`
          (goto _label_3 :!via `Reset`))))
    (:`then_1`
      (`KismetSystemLibrary.RetriggerableDelay` 1.0)
      (`|ExecutionSequence`
        (:`then_0`
          (goto _label_2 :!via `Reset`))
        (:`then_1`
          (`/Engine/EditorBlueprintResources/StandardMacros.DoOnce` false :!label _label_3
            (:`Completed`
              (bind _aichasemusic (`self.AIChaseMusic`)
                (:`then`
                  (`AudioComponent.FadeOut` _aichasemusic 1.0 0.0 "Linear")
                  (set `/Game/ThirdPerson/Blueprints/BP_ThirdPersonGameMode2.MusicPlaying?` false (`self.As BP Third Person Game Mode 2`)))
                (:`else`)))))))))

(event `Key|LeftMouseButton`
  (params (Key :type "Key Structure"))
  (bind _returnvalue (`self.K2_GetActorLocation`))
  (:`Pressed`
    (`/Engine/EditorBlueprintResources/StandardMacros.DoOnce` false :!label _label_4
      (:`Completed`
        (bind _returnvalue_2 (`self.PlayAnimMontage` "/Game/Characters/Main_Character/WithSword/mc_slash_anim_Montage.mc_slash_anim_Montage"))
        (`KismetSystemLibrary.Delay` _returnvalue_2)
        (`KismetSystemLibrary.SphereTraceSingleForObjects` :`Start` _returnvalue :`End` (+ _returnvalue (* (`self.GetActorForwardVector`) 150.0)) :`Radius` 30.0 :`ObjectTypes` (`|MakeArray` "ObjectTypeQuery3" :!type "EObjectTypeQuery Enum") :`DrawDebugType` "ForDuration" :`DrawTime` 1.0)
        (goto _label_4 :!via `Reset`)))))

(event `Death`
  (bind _returnvalue (`self.K2_GetActorLocation`))
  (bind _aichasemusic (`self.AIChaseMusic`)
    (:`then`
      (`AudioComponent.FadeOut` _aichasemusic 1.0 0.0 "Linear")
      (set `/Game/ThirdPerson/Blueprints/BP_ThirdPersonGameMode2.MusicPlaying?` false (`self.As BP Third Person Game Mode 2`))
      (`GameplayStatics.SpawnEmitterAtLocation` "/Game/Vefects/Zap_VFX/VFX/Zap/Particles/PS_Zap_02.PS_Zap_02" _returnvalue (struct) (7.0 7.0 7.0))
      (`GameplayStatics.SpawnSoundAtLocation` "/Engine/VREditor/Sounds/UI/Leave_Simulate.Leave_Simulate" _returnvalue (struct) 1.0 1.0 0.0 null null)
      (`self.K2_DestroyActor`)
      (bind _asbp_my_game_instance (cast `/Game/ThirdPerson/Blueprints/BP_MyGameInstance` (`GameplayStatics.GetGameInstance`)))
      (bind _moonbeetleskilled (`/Game/ThirdPerson/Blueprints/BP_MyGameInstance.AddMoonBeetleKill` _asbp_my_game_instance))
      (if (== _moonbeetleskilled 3)
        (bind _asbp_player_controller (cast `/Game/ThirdPerson/Blueprints/BP_PlayerController` (`GameplayStatics.GetPlayerController` 0)))
        (`/Game/ThirdPerson/Blueprints/BP_PlayerController.CompleteQuest` _asbp_player_controller "NewEnumerator2")
        (`GameplayStatics.PlaySound2D` "/Engine/EditorSounds/GamePreview/EjectFromPlayer_Cue.EjectFromPlayer_Cue" 1.0 1.0 0.0 null null)
        (`KismetSystemLibrary.Delay` 0.3)))
    (:`else`)))

(fn `GetCurrentHealth`
  (returns (Health :type "Float (double-precision)"))
  (return (`/Game/DamageSystem/BPC_DamageSystem.Health` (`self.BPC_DamageSystem`))))

(fn `GetMaxHealth`
  (returns (MaxHealth :type "Float (double-precision)"))
  (return (`/Game/DamageSystem/BPC_DamageSystem.MaxHealth` (`self.BPC_DamageSystem`))))

(fn `Heal`
  (params (Amount :type "Float (double-precision)"))
  (returns (NewHealth :type "Float (double-precision)"))
  (bind _newhealth (`/Game/DamageSystem/BPC_DamageSystem.Heal` (`self.BPC_DamageSystem`) Amount))
  (return _newhealth))

(fn `TakeDamage`
  (params (DamageInfo :type "/Game/DamageSystem/S_DamageInfo Structure"))
  (returns (WasDamaged :type Boolean))
  (bind _wasdamaged (`/Game/DamageSystem/BPC_DamageSystem.TakeDamage` (`self.BPC_DamageSystem`) DamageInfo))
  (return _wasdamaged))

(fn `UserConstructionScript`
  (add `/Game/DamageSystem/BPC_DamageSystem.OnDeath` (`self.BPC_DamageSystem`) (`|CreateDelegate` :!event `Death`)))