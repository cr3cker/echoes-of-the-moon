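; BP_PoisonousMushroom is a hazard that drains player health while something overlaps its Box.
; Begin overlap starts a fast looping timer that fires PoisonDamage, and end overlap clears it.
; Each tick of the timer subtracts Damage directly from PlayerHealth in BP_MyGameInstance.
; The overlap events do not filter the other actor, so any overlapping object can trigger the drain.
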(event `self.Box.OnComponentBeginOverlap`
  (params (OverlappedComponent :type "PrimitiveComponent Object Reference") (OtherActor :type "Actor Object Reference") (OtherComp :type "PrimitiveComponent Object Reference") (OtherBodyIndex :type Integer) (bFromSweep :type Boolean) (SweepResult :type "HitResult Structure (by ref)"))
  (bind _returnvalue (`KismetSystemLibrary.K2_SetTimerDelegate` (delegate `PoisonDamage`) 0.1 true))
  (set `self.DamageTimer` _returnvalue))

(event `PoisonDamage`
  (bind _asbp_my_game_instance (cast `/Game/ThirdPerson/Blueprints/BP_MyGameInstance` (`GameplayStatics.GetGameInstance`)))
  (set `/Game/ThirdPerson/Blueprints/BP_MyGameInstance.PlayerHealth` (- (`/Game/ThirdPerson/Blueprints/BP_MyGameInstance.PlayerHealth` _asbp_my_game_instance) (`self.Damage`)) _asbp_my_game_instance))

(event `self.Box.OnComponentEndOverlap`
  (params (OverlappedComponent :type "PrimitiveComponent Object Reference") (OtherActor :type "Actor Object Reference") (OtherComp :type "PrimitiveComponent Object Reference") (OtherBodyIndex :type Integer))
  (`KismetSystemLibrary.K2_ClearAndInvalidateTimerHandle` (`self.DamageTimer`)))

(fn `UserConstructionScript`)