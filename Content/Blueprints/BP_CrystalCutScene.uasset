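; BP_CrystalCutScene is a floating crystal pickup that the player collects by touching it.
; Two chained timelines move the mesh's relative location back and forth in a continuous loop, starting on BeginPlay.
; When an actor tagged Player overlaps the trigger, it plays a sound and zap particle effect, calls AddCrystals on BP_PlayerController, then destroys itself.
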(event `self.ReceiveBeginPlay`
  (bind (_direction _z_axis_movement) (`Timeline|Floating animation` :!label _label)
    (:`Update`
      (`SceneComponent.K2_SetRelativeLocation` (`self.Mesh`) _z_axis_movement false false))
    (:`Finished`
      (bind (_direction_2 _z_axis_movement_2) (`Timeline|Шкала времени` :!via `ReverseFromEnd`)
        (:`Update`
          (`SceneComponent.K2_SetRelativeLocation` (`self.Mesh`) _z_axis_movement_2 false false))
        (:`Finished`
          (goto _label :!via `PlayFromStart`))))))

(event `self.Trigger.OnComponentBeginOverlap`
  (params (OverlappedComponent :type "PrimitiveComponent Object Reference") (OtherActor :type "Actor Object Reference") (OtherComp :type "PrimitiveComponent Object Reference") (OtherBodyIndex :type Integer) (bFromSweep :type Boolean) (SweepResult :type "HitResult Structure (by ref)"))
  (bind _returnvalue (`self.K2_GetActorLocation`))
  (if (`self.ActorHasTag` OtherActor "Player")
    (`GameplayStatics.PlaySoundAtLocation` "/Engine/VREditor/Sounds/UI/Floating_UI_Open-002.Floating_UI_Open-002" _returnvalue (struct) 1.0 1.0 0.0 null null null null)
    (`GameplayStatics.SpawnEmitterAtLocation` "/Game/Vefects/Zap_VFX/VFX/Zap/Particles/PS_Zap_02.PS_Zap_02" _returnvalue (struct) (2.0 2.0 2.0) true "AutoRelease")
    (bind _asbp_player_controller (cast `/Game/ThirdPerson/Blueprints/BP_PlayerController` (`GameplayStatics.GetPlayerController` 0)))
    (`/Game/ThirdPerson/Blueprints/BP_PlayerController.AddCrystals` _asbp_player_controller)
    (`self.K2_DestroyActor`)))

(fn `UserConstructionScript`)