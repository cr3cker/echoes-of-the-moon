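; BP_Duck is an ambient NPC duck that wanders by alternating timed walking and idle phases.
; A self-restarting, Delay-based LoopAnim toggles Walking, passes speed to the ABP_Birds anim instance, then turns the duck 45 degrees after each pause.
; MoveTick, apparently driven by a fast looping timer instead of Tick, sweeps it forward while walking.
; FlipDirection also negates Direction, but movement ignores that value.
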(event `self.ReceiveBeginPlay`
  (`KismetSystemLibrary.K2_SetTimerDelegate` (`|CreateDelegate` :!event `MoveTick`) 0.08 true)
  (`self.LoopAnim`))

(event `MoveTick`
  (if (`self.bWalking`)
    (`self.K2_AddActorWorldOffset` (* (`self.GetActorForwardVector`) (`self.WalkSpeed`) (`GameplayStatics.GetWorldDeltaSeconds`) (`self.number`)) true)))

(event `SetSpeed`
  (bind _asabp_birds (cast `/Game/Blueprints/NPC/ABP_Birds` (`SkeletalMeshComponent.GetAnimInstance` (`self.Mesh`))))
  (if (`self.bWalking`)
    (set `/Game/Blueprints/NPC/ABP_Birds.Speed` (`self.WalkSpeed`) _asabp_birds)
    (else
      (set `/Game/Blueprints/NPC/ABP_Birds.Speed` 0.0 _asabp_birds))))

(event `LoopAnim`
  (set `self.bWalking` true)
  (`self.SetSpeed`)
  (`KismetSystemLibrary.Delay` 7.0)
  (set `self.bWalking` false)
  (`self.SetSpeed`)
  (`KismetSystemLibrary.Delay` 4.0)
  (`self.FlipDirection`)
  (`self.LoopAnim`))

(event `FlipDirection`
  (set `self.Direction` (* (`self.Direction`) -1.0))
  (`self.K2_AddActorWorldRotation` (struct :`Yaw` 45.0)))

(fn `UserConstructionScript`)