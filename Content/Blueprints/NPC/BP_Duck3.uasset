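; Duck NPC that wanders and flees when its pawn sensing spots a pawn.
; A delay loop alternates walking and idling with 90-degree turns, ending if the duck is fleeing at the turn check.
; Sighting triggers a timed 180-degree run, while SetSpeed feeds movement state to the ABP_Birds animation blueprint.
; MoveTick applies swept forward offsets; a looping timer starts at BeginPlay.
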(event `self.ReceiveBeginPlay`
  (`KismetSystemLibrary.K2_SetTimerDelegate` (`|CreateDelegate` :!event `MoveTick`) 0.08 true)
  (`self.LoopAnim`))

(event `MoveTick`
  (if (`self.bRunningAway`)
    (`self.K2_AddActorWorldOffset` (* (`self.RunSpeed`) (`self.GetActorForwardVector`) (`GameplayStatics.GetWorldDeltaSeconds`) (`self.number`)) true)
    (elif (`self.bWalking`)
      (`self.K2_AddActorWorldOffset` (* (`self.GetActorForwardVector`) (`self.WalkSpeed`) (`GameplayStatics.GetWorldDeltaSeconds`) (`self.number`)) true))))

(event `SetSpeed`
  (bind _asabp_birds (cast `/Game/Blueprints/NPC/ABP_Birds` (`SkeletalMeshComponent.GetAnimInstance` (`self.Mesh`))))
  (if (`self.bWalking`)
    (set `/Game/Blueprints/NPC/ABP_Birds.Speed` (`self.WalkSpeed`) _asabp_birds)
    (elif (`self.bRunningAway`)
      (set `/Game/Blueprints/NPC/ABP_Birds.Speed` 700.0 _asabp_birds)
      (else
        (set `/Game/Blueprints/NPC/ABP_Birds.Speed` 0.0 _asabp_birds)))))

(event `LoopAnim`
  (set `self.bWalking` true)
  (`self.SetSpeed`)
  (`KismetSystemLibrary.Delay` 5.0)
  (set `self.bWalking` false)
  (`self.SetSpeed`)
  (`KismetSystemLibrary.Delay` 4.0)
  (if (not (`self.bRunningAway`))
    (`self.FlipDirection`)
    (`self.LoopAnim`)))

(event `FlipDirection`
  (set `self.Direction` (* (`self.Direction`) -1.0))
  (`self.K2_AddActorWorldRotation` (struct :`Yaw` 90.0)))

(event `self.PawnSensing.OnSeePawn`
  (params (Pawn :type "Pawn Object Reference"))
  (if (not (`self.bRunningAway`))
    (`self.RunAway`)))

(event `RunAway`
  (set `self.bWalking` false)
  (set `self.bRunningAway` true)
  (`self.K2_AddActorWorldRotation` (struct :`Yaw` 180.0))
  (`self.SetSpeed`)
  (`KismetSystemLibrary.Delay` (`self.RunDuration`))
  (set `self.bRunningAway` false)
  (set `self.bWalking` true))

(fn `UserConstructionScript`)