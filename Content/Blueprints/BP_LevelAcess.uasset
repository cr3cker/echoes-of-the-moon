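; Double-door gate that gives access to the Forest1 level.
; StartGateEvent calls OpenDoor, which runs two timelines that swing the right and left doors 120 degrees in opposite directions and flag the gate as open.
; Once open, any end overlap on the Box, with no actor check, plays a camera shutter sound and loads Forest1 after a short delay.
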(event `Open Door`
  (`|ExecutionSequence`
    (:`then_0`
      (bind (_direction _doorfloat) (`Timeline|Timeline` :!via `PlayFromStart`)
        (:`Update`
          (`SceneComponent.K2_SetRelativeRotation` (`self.DoorR`) (`KismetMathLibrary.MakeRotator` 0.0 0.0 (`KismetMathLibrary.Lerp` 0.0 -120.0 _doorfloat)) false false))))
    (:`then_1`
      (bind (_direction_2 _doorfloat_2) (`Timeline|OpenDoor` :!via `PlayFromStart`)
        (:`Update`
          (`SceneComponent.K2_SetRelativeRotation` (`self.DoorL`) (`KismetMathLibrary.MakeRotator` 0.0 0.0 (`KismetMathLibrary.Lerp` 0.0 120.0 _doorfloat_2)) false false)
          (set `self.DoorOpen?` true))))))

(event `self.Box.OnComponentEndOverlap`
  (params (OverlappedComponent :type "PrimitiveComponent Object Reference") (OtherActor :type "Actor Object Reference") (OtherComp :type "PrimitiveComponent Object Reference") (OtherBodyIndex :type Integer))
  (if (`self.DoorOpen?`)
    (`GameplayStatics.PlaySound2D` "/Engine/VREditor/Sounds/UI/Camera_Shutter.Camera_Shutter" 1.0 1.0 0.0 null null)
    (`KismetSystemLibrary.Delay` 0.25)
    (`GameplayStatics.OpenLevel` "Forest1")))

(fn `StartGateEvent`
  (`self.Open Door`))

(fn `UserConstructionScript`)