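; BP_RespawnPoint is an interactable checkpoint that saves the player's respawn location.
; Overlapping its sphere shows a prompt widget while unsaved and arms the IA_Interaction input, which the actor receives by enabling input on BeginPlay.
; Interacting plays a sound, rescales and relights Sphere1, hides the prompt, and marks the point saved.
; It then stores the player's transform, current level name and a saved flag in BP_MyGameInstance.
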(event `self.Sphere.OnComponentBeginOverlap`
  (params (OverlappedComponent :type "PrimitiveComponent Object Reference") (OtherActor :type "Actor Object Reference") (OtherComp :type "PrimitiveComponent Object Reference") (OtherBodyIndex :type Integer) (bFromSweep :type Boolean) (SweepResult :type "HitResult Structure (by ref)"))
  (if (not (`self.Saved?`))
    (`SceneComponent.SetVisibility` (`self.Widget`) true false)
    (set `self.CanSave` true)))

(event `self.Sphere.OnComponentEndOverlap`
  (params (OverlappedComponent :type "PrimitiveComponent Object Reference") (OtherActor :type "Actor Object Reference") (OtherComp :type "PrimitiveComponent Object Reference") (OtherBodyIndex :type Integer))
  (`SceneComponent.SetVisibility` (`self.Widget`) false false)
  (set `self.CanSave` false))

(event `EnhancedInput|/Game/ThirdPerson/Input/Actions/IA_Interaction`
  (params (ActionValue :type Boolean) (ElapsedSeconds :type "Float (double-precision)") (TriggeredSeconds :type "Float (double-precision)") (InputAction :type "InputAction Object Reference" :default "/Game/ThirdPerson/Input/Actions/IA_Interaction.IA_Interaction"))
  (:`Started`
    (if (`self.CanSave`)
      (`GameplayStatics.SpawnSoundAtLocation` "/Engine/EditorSounds/GamePreview/StartSimulate.StartSimulate" (0.0 0.0 0.0) (struct) 1.0 1.0 0.0 null null)
      (`SceneComponent.SetWorldScale3D` (`self.Sphere1`) (0.65 0.65 0.65))
      (`PrimitiveComponent.SetMaterial` (`self.Sphere1`) 0 "/Game/CR/LQ/AMT_Materials/MI_Light_4_2.MI_Light_4_2")
      (set `self.Saved?` true)
      (`SceneComponent.SetVisibility` (`self.Widget`) false false)
      (bind _asbp_my_game_instance (cast `/Game/ThirdPerson/Blueprints/BP_MyGameInstance` (`GameplayStatics.GetGameInstance`)))
      (set `/Game/ThirdPerson/Blueprints/BP_MyGameInstance.SavedRespawnTransform` (`self.GetTransform` (`GameplayStatics.GetPlayerCharacter` 0)) _asbp_my_game_instance)
      (set `/Game/ThirdPerson/Blueprints/BP_MyGameInstance.HaveSavedRespawn` true _asbp_my_game_instance)
      (bind _returnvalue (`GameplayStatics.GetCurrentLevelName` true))
      (set `/Game/ThirdPerson/Blueprints/BP_MyGameInstance.SavedRespawnLevelName` (`KismetStringLibrary.Conv_StringToName` _returnvalue) _asbp_my_game_instance)
      (`KismetSystemLibrary.PrintString` _returnvalue))))

(event `self.ReceiveBeginPlay`
  (`self.EnableInput` (`GameplayStatics.GetPlayerController` 0)))

(fn `UserConstructionScript`)