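; BP_Friend is an AI pawn that moves toward pawns it sees and can take damage or be healed.
; PawnSensing sightings trigger ChasePlayer, which runs AI Move To on the seen pawn.
; A retriggerable delay flips two DoOnce gates when sightings lapse, though neither gate drives further logic.
; Health queries, Heal and TakeDamage delegate to BPCDamageSystem, and BeginPlay caches the third-person game mode.
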(event `self.ReceiveBeginPlay`
  (bind _asbp_third_person_game_mode_2 (cast `/Game/ThirdPerson/Blueprints/BP_ThirdPersonGameMode2` (`GameplayStatics.GetGameMode`)))
  (set `self.As BP Third Person Game Mode 2` _asbp_third_person_game_mode_2))

(event `ChasePlayer`
  (params (TargetPawn :type "Pawn Object Reference"))
  (`|AIMoveTo` self (0.0 0.0 0.0) TargetPawn 10.0))

(event `self.PawnSensing.OnSeePawn`
  (params (Pawn :type "Pawn Object Reference"))
  (`|ExecutionSequence`
    (:`then_0`
      (`self.ChasePlayer` Pawn)
      (`|ExecutionSequence`
        (:`then_0`
          (`/Engine/EditorBlueprintResources/StandardMacros.DoOnce` false :!label _label))
        (:`then_1`
          (goto _label_2 :!via `Reset`))))
    (:`then_1`
      (`KismetSystemLibrary.RetriggerableDelay` 1.0)
      (`|ExecutionSequence`
        (:`then_0`
          (goto _label :!via `Reset`))
        (:`then_1`
          (`/Engine/EditorBlueprintResources/StandardMacros.DoOnce` false :!label _label_2))))))

(fn `GetCurrentHealth`
  (returns (Health :type "Float (double-precision)"))
  (return (`/Game/DamageSystem/BPC_DamageSystem.Health` (`self.BPC_DamageSystem`))))

(fn `GetMaxHealth`
  (returns (MaxHealth :type "Float (double-precision)"))
  (return (`/Game/DamageSystem/BPC_DamageSystem.MaxHealth` (`self.BPC_DamageSystem`))))

(fn `Heal`
  (params (Amount :type "Float (double-precision)"))
  (returns (NewHealth :type "Float (double-precision)"))
  (bind _newhealth (`/Game/DamageSystem/BPC_DamageSystem.Heal` (`self.BPC_DamageSystem`) Amount))
  (return _newhealth))

(fn `TakeDamage`
  (params (DamageInfo :type "/Game/DamageSystem/S_DamageInfo Structure"))
  (returns (WasDamaged :type Boolean))
  (bind _wasdamaged (`/Game/DamageSystem/BPC_DamageSystem.TakeDamage` (`self.BPC_DamageSystem`) DamageInfo))
  (return _wasdamaged))

(fn `UserConstructionScript`)