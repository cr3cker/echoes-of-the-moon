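; Enemy AI character that chases any pawn it sees via PawnSensing and AIMoveTo.
; Health, Heal and TakeDamage functions forward to BPCDamageSystem, whose OnDeath is bound in the construction script.
; Death spawns an effect and sound, hides the mesh and sets it to query-only collision.
; A left-mouse test attack plays a DoOnce-gated slash montage, then runs a debug-drawn forward sphere trace without applying damage.
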(event `ChasePlayer`
  (params (TargetPawn :type "Pawn Object Reference"))
  (`|AIMoveTo` self (0.0 0.0 0.0) TargetPawn 250.0))

(event `self.PawnSensing.OnSeePawn`
  (params (Pawn :type "Pawn Object Reference"))
  (`self.ChasePlayer` Pawn))

(event `Key|LeftMouseButton`
  (params (Key :type "Key Structure"))
  (bind _returnvalue (`self.K2_GetActorLocation`))
  (:`Pressed`
    (`/Engine/EditorBlueprintResources/StandardMacros.DoOnce` false :!label _label
      (:`Completed`
        (bind _returnvalue_2 (`self.PlayAnimMontage` "/Game/Characters/Main_Character/WithSword/mc_slash_anim_Montage.mc_slash_anim_Montage"))
        (`KismetSystemLibrary.Delay` _returnvalue_2)
        (`KismetSystemLibrary.SphereTraceSingleForObjects` :`Start` _returnvalue :`End` (+ _returnvalue (* (`self.GetActorForwardVector`) 150.0)) :`Radius` 30.0 :`ObjectTypes` (`|MakeArray` "ObjectTypeQuery3" :!type "EObjectTypeQuery Enum") :`DrawDebugType` "ForDuration" :`DrawTime` 1.0)
        (goto _label :!via `Reset`)))))

(event `Death`
  (bind _returnvalue (`self.K2_GetActorLocation`))
  (bind _mesh (`self.Mesh`))
  (`GameplayStatics.SpawnEmitterAtLocation` "/Game/Vefects/Zap_VFX/VFX/Zap/Particles/PS_Zap_02.PS_Zap_02" _returnvalue (struct) (7.0 7.0 7.0))
  (`GameplayStatics.SpawnSoundAtLocation` "/Engine/VREditor/Sounds/UI/Leave_Simulate.Leave_Simulate" _returnvalue (struct) 1.0 1.0 0.0 null null)
  (`SceneComponent.SetVisibility` _mesh false true)
  (`PrimitiveComponent.SetCollisionEnabled` _mesh "QueryOnly"))

(fn `GetCurrentHealth`
  (returns (Health :type "Float (double-precision)"))
  (return (`/Game/DamageSystem/BPC_DamageSystem.Health` (`self.BPC_DamageSystem`))))

(fn `GetMaxHealth`
  (returns (MaxHealth :type "Float (double-precision)"))
  (return (`/Game/DamageSystem/BPC_DamageSystem.MaxHealth` (`self.BPC_DamageSystem`))))

(fn `Heal`
  (params (Amount :type "Float (double-precision)"))
  (returns (NewHealth :type "Float (double-precision)"))
  (bind _newhealth (`/Game/DamageSystem/BPC_DamageSystem.Heal` (`self.BPC_DamageSystem`) Amount))
  (return _newhealth))

(fn `TakeDamage`
  (params (DamageInfo :type "/Game/DamageSystem/S_DamageInfo Structure"))
  (returns (WasDamaged :type Boolean))
  (bind _wasdamaged (`/Game/DamageSystem/BPC_DamageSystem.TakeDamage` (`self.BPC_DamageSystem`) DamageInfo))
  (return _wasdamaged))

(fn `UserConstructionScript`
  (add `/Game/DamageSystem/BPC_DamageSystem.OnDeath` (`self.BPC_DamageSystem`) (`|CreateDelegate` :!event `Death`)))