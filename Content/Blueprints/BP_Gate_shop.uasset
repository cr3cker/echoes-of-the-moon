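; BP_Gate_shop is a trigger gate that sends the player to the Shop level.
; On box overlap by the third-person character, it saves the player's transform in the game instance, keyed by current level name.
; It then plays a camera shutter sound, waits briefly, destroys itself and opens Shop.
; A DoOnce with a delayed reset throttles retriggering, though any overlapping actor consumes it before the character cast.
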(event `self.Box.OnComponentBeginOverlap`
  (params (OverlappedComponent :type "PrimitiveComponent Object Reference") (OtherActor :type "Actor Object Reference") (OtherComp :type "PrimitiveComponent Object Reference") (OtherBodyIndex :type Integer) (bFromSweep :type Boolean) (SweepResult :type "HitResult Structure (by ref)"))
  (`/Engine/EditorBlueprintResources/StandardMacros.DoOnce` false :!label _label
    (:`Completed`
      (`|ExecutionSequence`
        (:`then_0`
          (bind _asbp_third_person_character (cast `/Game/ThirdPerson/Blueprints/BP_ThirdPersonCharacter` OtherActor))
          (bind _asbp_my_game_instance (cast `/Game/ThirdPerson/Blueprints/BP_MyGameInstance` (`GameplayStatics.GetGameInstance`)))
          (bind _returnvalue (`GameplayStatics.GetCurrentLevelName` true))
          (`BlueprintMapLibrary.Map_Add` (`/Game/ThirdPerson/Blueprints/BP_MyGameInstance.SavedPlayerTransforms` _asbp_my_game_instance) _returnvalue (`self.GetTransform` _asbp_third_person_character))
          (`GameplayStatics.PlaySound2D` "/Engine/VREditor/Sounds/UI/Camera_Shutter.Camera_Shutter" 1.0 1.0 0.0 null null)
          (`KismetSystemLibrary.Delay` 0.25)
          (`self.K2_DestroyActor`)
          (`GameplayStatics.OpenLevel` "Shop"))
        (:`then_1`
          (`KismetSystemLibrary.Delay` 10.0)
          (goto _label :!via `Reset`))))))

(fn `UserConstructionScript`)