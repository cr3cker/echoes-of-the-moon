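; BP_RespawnCheckpoint is a checkpoint actor that offers an interaction prompt for saving while something overlaps its sphere.
; Begin and end overlap on Sphere1 toggle the widget's visibility and the CanSave flag, with no filter on the overlapping actor.
; It enables input from player controller 0 on BeginPlay, so IA_Interaction reaches it directly.
; Interacting while CanSave is true only prints "Saved"; no save or respawn logic is implemented.
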(event `self.Sphere1.OnComponentBeginOverlap`
  (params (OverlappedComponent :type "PrimitiveComponent Object Reference") (OtherActor :type "Actor Object Reference") (OtherComp :type "PrimitiveComponent Object Reference") (OtherBodyIndex :type Integer) (bFromSweep :type Boolean) (SweepResult :type "HitResult Structure (by ref)"))
  (`SceneComponent.SetVisibility` (`self.Widget`) true false)
  (set `self.CanSave` true)
  (`KismetSystemLibrary.PrintString` "CanSave"))

(event `self.Sphere1.OnComponentEndOverlap`
  (params (OverlappedComponent :type "PrimitiveComponent Object Reference") (OtherActor :type "Actor Object Reference") (OtherComp :type "PrimitiveComponent Object Reference") (OtherBodyIndex :type Integer))
  (`SceneComponent.SetVisibility` (`self.Widget`) false false)
  (set `self.CanSave` false))

(event `EnhancedInput|/Game/ThirdPerson/Input/Actions/IA_Interaction`
  (params (ActionValue :type Boolean) (ElapsedSeconds :type "Float (double-precision)") (TriggeredSeconds :type "Float (double-precision)") (InputAction :type "InputAction Object Reference" :default "/Game/ThirdPerson/Input/Actions/IA_Interaction.IA_Interaction"))
  (:`Started`
    (if (`self.CanSave`)
      (`KismetSystemLibrary.PrintString` "Saved"))))

(event `self.ReceiveBeginPlay`
  (`self.EnableInput` (`GameplayStatics.GetPlayerController` 0)))

(fn `UserConstructionScript`)