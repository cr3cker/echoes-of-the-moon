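; BP_MasterItem is an interactable item that sends the player to the Shop level.
; Sphere overlap toggles widgets, an animated UI_Interact prompt, an outline overlay and CanPressE.
; CanRecieveTrace can also show the hint, but its hide branch is unreachable behind a repeated CanInteract check.
; The interaction input, guarded by a resetting DoOnce, saves the player transform per level in the GameInstance, completes a quest and opens Shop after timed sounds.
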(event `self.Sphere.OnComponentBeginOverlap`
  (params (OverlappedComponent :type "PrimitiveComponent Object Reference") (OtherActor :type "Actor Object Reference") (OtherComp :type "PrimitiveComponent Object Reference") (OtherBodyIndex :type Integer) (bFromSweep :type Boolean) (SweepResult :type "HitResult Structure (by ref)"))
  (bind _widget (`self.Widget`))
  (`SceneComponent.SetVisibility` (`self.Widget1`) true false)
  (set `self.CanPressE` true)
  (cast `/Game/ThirdPerson/Blueprints/BP_ThirdPersonCharacter` OtherActor)
  (if (`self.CanInteract`)
    (bind _returnvalue (`|CreateWidget` "/Game/Interaction_promt/UI_Interact.UI_Interact_C"))
    (bind _output_get (set `self.Interaction Widget` _returnvalue))
    (`WidgetComponent.SetWidget` _widget _output_get)
    (`SceneComponent.SetVisibility` _widget true false)
    (bind _interaction_widget (`self.Interaction Widget`)
      (:`then`
        (if (not (`self.HintVisible`))
          (`UserWidget.PlayAnimation` _interaction_widget (`/Game/Interaction_promt/UI_Interact.PopUp` _interaction_widget) 0.0 1 "Forward" 1.5 false)
          (set `self.HintVisible` true)
          (`MeshComponent.SetOverlayMaterial` (`self.StaticMesh`) "/Game/Interaction_promt/M_Outline.M_Outline")
          (set `self.CanPressE` true)))
      (:`else`))))

(event `self.Sphere.OnComponentEndOverlap`
  (params (OverlappedComponent :type "PrimitiveComponent Object Reference") (OtherActor :type "Actor Object Reference") (OtherComp :type "PrimitiveComponent Object Reference") (OtherBodyIndex :type Integer))
  (`SceneComponent.SetVisibility` (`self.Widget1`) false false)
  (set `self.CanPressE` false)
  (cast `/Game/ThirdPerson/Blueprints/BP_ThirdPersonCharacter` OtherActor)
  (if (`self.CanInteract`)
    (bind _interaction_widget (`self.Interaction Widget`)
      (:`then`
        (if (`self.HintVisible`)
          (`UserWidget.PlayAnimation` _interaction_widget (`/Game/Interaction_promt/UI_Interact.PopUp` _interaction_widget) 0.0 1 "Forward" 1.5 false)
          (set `self.HintVisible` false)
          (set `self.CanPressE` false)
          (`MeshComponent.SetOverlayMaterial` (`self.StaticMesh`) null))
        (`KismetSystemLibrary.Delay` 0.15)
        (`Widget.RemoveFromParent` (`self.Interaction Widget`))
        (set `self.Interaction Widget` null)
        (`SceneComponent.SetVisibility` (`self.Widget`) false false))
      (:`else`))))

(event `/Game/Blueprints/BPI_Interaction.Can RecieveTrace`
  (params (CanInteract :type Boolean))
  (if (`self.CanInteract`)
    (if CanInteract
      (bind _interaction_widget (`self.Interaction Widget`)
        (:`then`
          (if (not (`self.HintVisible`))
            (`UserWidget.PlayAnimation` _interaction_widget (`/Game/Interaction_promt/UI_Interact.PopUp` _interaction_widget) 0.0 1 "Forward" 1.5 false)
            (set `self.HintVisible` true)
            (`MeshComponent.SetOverlayMaterial` (`self.StaticMesh`) "/Game/Interaction_promt/M_Outline.M_Outline")
            (set `self.CanPressE` true)))
        (:`else`))
      (else
        (bind _interaction_widget_2 (`self.Interaction Widget`)
          (:`then`
            (if (not (`self.HintVisible`))
              (`UserWidget.PlayAnimation` _interaction_widget_2 (`/Game/Interaction_promt/UI_Interact.PopUp` _interaction_widget_2) 0.0 1 "Reverse" 1.5 false)
              (set `self.HintVisible` false)
              (`MeshComponent.SetOverlayMaterial` (`self.StaticMesh`) null)
              (set `self.CanPressE` false)))
          (:`else`))))))

(event `EnhancedInput|/Game/ThirdPerson/Input/Actions/IA_Interaction`
  (params (ActionValue :type Boolean) (ElapsedSeconds :type "Float (double-precision)") (TriggeredSeconds :type "Float (double-precision)") (InputAction :type "InputAction Object Reference" :default "/Game/ThirdPerson/Input/Actions/IA_Interaction.IA_Interaction"))
  (:`Started`
    (if (`self.CanPressE`)
      (`/Engine/EditorBlueprintResources/StandardMacros.DoOnce` false :!label _label
        (:`Completed`
          (`|ExecutionSequence`
            (:`then_0`
              (bind _asbp_third_person_character (cast `/Game/ThirdPerson/Blueprints/BP_ThirdPersonCharacter` (`GameplayStatics.GetPlayerCharacter` 0)))
              (bind _asbp_my_game_instance (cast `/Game/ThirdPerson/Blueprints/BP_MyGameInstance` (`GameplayStatics.GetGameInstance`)))
              (bind _returnvalue (`GameplayStatics.GetCurrentLevelName` true))
              (`BlueprintMapLibrary.Map_Add` (`/Game/ThirdPerson/Blueprints/BP_MyGameInstance.SavedPlayerTransforms` _asbp_my_game_instance) _returnvalue (`self.GetTransform` _asbp_third_person_character))
              (bind _asbp_player_controller (cast `/Game/ThirdPerson/Blueprints/BP_PlayerController` (`GameplayStatics.GetPlayerController` 0)))
              (`GameplayStatics.PlaySound2D` "/Engine/EditorSounds/GamePreview/EjectFromPlayer_Cue.EjectFromPlayer_Cue" 1.0 1.0 0.0 null null)
              (`KismetSystemLibrary.Delay` 0.7)
              (`/Game/ThirdPerson/Blueprints/BP_PlayerController.CompleteQuest` _asbp_player_controller "NewEnumerator0")
              (`GameplayStatics.PlaySound2D` "/Engine/VREditor/Sounds/UI/Camera_Shutter.Camera_Shutter" 1.0 1.0 0.0 null null)
              (`KismetSystemLibrary.Delay` 0.25)
              (`GameplayStatics.OpenLevel` "Shop"))
            (:`then_1`
              (`KismetSystemLibrary.Delay` 10.0)
              (goto _label :!via `Reset`))))))))

(event `self.ReceiveBeginPlay`
  (`self.EnableInput` (`GameplayStatics.GetPlayerController` 0)))

(fn `UserConstructionScript`)